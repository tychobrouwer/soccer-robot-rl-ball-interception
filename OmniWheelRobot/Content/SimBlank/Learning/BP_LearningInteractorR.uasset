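; Learning Agents interactor that connects an OmniRobot agent to a policy in a robot-and-ball simulation.
; It observes the robot's global velocity, ball velocity, and ball location offset from the robot body's position.
; The action pairs a three-way discrete acceleration choice with a direction angle, written to the robot's setpoint variables along with a time delta.
; Heading, max-limit and other observation nodes remain unconnected.
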(fn `GatherAgentObservation`
  (params (InObservationObject :type "LearningAgentsObservationObject Object Reference") (AgentId :type Integer))
  (returns (OutObservationObjectElement :type "LearningAgentsObservationObjectElement Structure"))
  (bind _output_get (set `self.obsActor` (`self.GetAgent` AgentId "/Game/SimBlank/Blueprints/OmniRobot.OmniRobot_C")))
  (set `self.Accurate-body` (`/Game/SimBlank/Blueprints/OmniRobot.accurate-body` _output_get))
  (return (`LearningAgentsObservations.MakeStructObservation` (`local.InObservationObject`) (`|MakeMap` "robotVelocity" (`LearningAgentsObservations.MakeVelocityObservation` (`local.InObservationObject`) (`/Game/SimBlank/Blueprints/OmniRobot.globalSpeed` (`self.obsActor`)) (`KismetMathLibrary.MakeTransform` (0.0 0.0 0.0)) "VelocityObservation" false null) "Ball" (`LearningAgentsObservations.MakeStructObservation` (`local.InObservationObject`) (`|MakeMap` "Location" (`LearningAgentsObservations.MakeLocationObservation` (`local.InObservationObject`) (`/Game/SimBlank/Blueprints/OmniRobot.ballLocation` (`self.obsActor`)) (`KismetMathLibrary.MakeTransform` (`SceneComponent.K2_GetComponentLocation` (`self.Accurate-body`))) "LocationObservation" false null) "Velocity" (`LearningAgentsObservations.MakeVelocityObservation` (`local.InObservationObject`) (`/Game/SimBlank/Blueprints/OmniRobot.ballVelocity` (`self.obsActor`)) (`KismetMathLibrary.MakeTransform` (0.0 0.0 0.0)) "VelocityObservation" false null) :!type "Name")) :!type "Name"))))

(fn `PerformAgentAction`
  (params (InActionObject :type "LearningAgentsActionObject Object Reference") (InActionObjectElement :type "LearningAgentsActionObjectElement Structure (by ref)") (AgentId :type Integer))
  (bind _actactor (`self.actActor`))
  (set `self.actActor` (`self.GetAgent` AgentId "/Game/SimBlank/Blueprints/OmniRobot.OmniRobot_C"))
  (bind _outelements (`LearningAgentsActions.GetStructAction` (`local.InActionObject`) (`local.InActionObjectElement`)))
  (`|ExecutionSequence`
    (:`then_0`
      (bind _outindex (`LearningAgentsActions.GetExclusiveDiscreteAction` (`local.InActionObject`) (`BlueprintMapLibrary.Map_Find` _outelements "acceleration") "DiscreteExclusiveAction" false null)))
    (:`then_1`
      (bind _outangle (`LearningAgentsActions.GetAngleActionRadians` (`local.InActionObject`) (`BlueprintMapLibrary.Map_Find` _outelements "direction") 0.0 "AngleAction" false null))
      (set `/Game/SimBlank/Blueprints/OmniRobot.genDirection` _outangle _actactor)
      (set `/Game/SimBlank/Blueprints/OmniRobot.genAccelaration` _outindex _actactor)
      (set `/Game/SimBlank/Blueprints/OmniRobot.tDeltaSetpoint` (`self.interferenceDeltaT`) _actactor)
      (return))))

(fn `SpecifyAgentAction`
  (params (InActionSchema :type "LearningAgentsActionSchema Object Reference"))
  (returns (OutActionSchemaElement :type "LearningAgentsActionSchemaElement Structure"))
  (return (`LearningAgentsActions.SpecifyStructAction` (`local.InActionSchema`) (`|MakeMap` "acceleration" (`LearningAgentsActions.SpecifyExclusiveDiscreteAction` (`local.InActionSchema`) 3) "direction" (`LearningAgentsActions.SpecifyAngleAction` (`local.InActionSchema`)) :!type "Name"))))

(fn `SpecifyAgentObservation`
  (params (InObservationSchema :type "LearningAgentsObservationSchema Object Reference"))
  (returns (OutObservationSchemaElement :type "LearningAgentsObservationSchemaElement Structure"))
  (return (`LearningAgentsObservations.SpecifyStructObservation` (`local.InObservationSchema`) (`|MakeMap` "robotVelocity" (`LearningAgentsObservations.SpecifyVelocityObservation` (`local.InObservationSchema`)) "Ball" (`LearningAgentsObservations.SpecifyStructObservation` (`local.InObservationSchema`) (`|MakeMap` "Location" (`LearningAgentsObservations.SpecifyLocationObservation` (`local.InObservationSchema`)) "Velocity" (`LearningAgentsObservations.SpecifyVelocityObservation` (`local.InObservationSchema`)) :!type "Name")) :!type "Name"))))