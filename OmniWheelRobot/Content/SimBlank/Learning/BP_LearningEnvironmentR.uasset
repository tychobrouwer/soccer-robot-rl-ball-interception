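; Learning Agents training environment that teaches OmniRobot agents to drive to a ball and stop on it.
; Reward combines exponential distance shaping, a large bonus for being close and nearly still, and an exponential time penalty normalised by starting ball distance.
; Episodes terminate on timeout, straying too far, or being close with low speed towards the ball.
; Reset increments the robot's training iteration, zeroes its timer and triggers its training reset.
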(fn `GatherAgentCompletion`
  (params (AgentId :type Integer))
  (returns (OutCompletion :type "ELearningAgentsCompletion Enum"))
  (locals (speedTowardsBallC :type "Float (double-precision)" :default 0.0) (distanceToBallC :type "Float (double-precision)" :default 0.0))
  (bind _returnvalue (`self.GetAgent` AgentId "/Game/SimBlank/Blueprints/OmniRobot.OmniRobot_C"))
  (bind _speedtowardsball (`/Game/SimBlank/Blueprints/OmniRobot.getSpeedTowardsBall` _returnvalue))
  (set `local.speedTowardsBallC` _speedtowardsball)
  (set `local.distanceToBallC` (`KismetMathLibrary.VSize` (- (`SceneComponent.K2_GetComponentLocation` (`/Game/SimBlank/Blueprints/OmniRobot.accurate-body` _returnvalue)) (`/Game/SimBlank/Blueprints/OmniRobot.ballLocation` _returnvalue))))
  (return (`LearningAgentsCompletions.CompletionOr` (`LearningAgentsCompletions.MakeCompletionOnTimeElapsed` (`/Game/SimBlank/Blueprints/OmniRobot.time` _returnvalue) 20.0 "Termination" "TimeElapsedCompletion" false null) (`LearningAgentsCompletions.MakeCompletionOnCondition` (> (`local.distanceToBallC`) 1000.0) "Termination" "ConditionCompletion" false null) (`LearningAgentsCompletions.MakeCompletionOnCondition` (and (< (`local.distanceToBallC`) 2.0) (< (`local.speedTowardsBallC`) 0.05)) "Termination" "ConditionCompletion" false null) "Running")))

(fn `GatherAgentReward`
  (params (AgentId :type Integer))
  (returns (OutReward :type "Float (single-precision)"))
  (locals (rewardActor :type "/Game/SimBlank/Blueprints/OmniRobot Object Reference") (speedTowardsBallR :type "Float (double-precision)" :default 0.0) (distanceToBallR :type "Float (double-precision)" :default 0.0))
  (bind _rewardactor (`local.rewardActor`))
  (bind _rewardactor_2 (`local.rewardActor`))
  (bind _returnvalue (and (< (`local.distanceToBallR`) 2.1) (< (`KismetMathLibrary.Abs` (`local.speedTowardsBallR`)) 0.06)))
  (bind _output_get (set `local.rewardActor` (`self.GetAgent` AgentId "/Game/SimBlank/Blueprints/OmniRobot.OmniRobot_C")))
  (bind _speedtowardsball (`/Game/SimBlank/Blueprints/OmniRobot.getSpeedTowardsBall` _output_get))
  (set `local.speedTowardsBallR` _speedtowardsball)
  (set `local.distanceToBallR` (`KismetMathLibrary.VSize` (- (`SceneComponent.K2_GetComponentLocation` (`/Game/SimBlank/Blueprints/OmniRobot.accurate-body` _rewardactor)) (`/Game/SimBlank/Blueprints/OmniRobot.ballLocation` _rewardactor))))
  (if _returnvalue
    (`KismetSystemLibrary.PrintText` null (`|FormatText` "Considered Success - {agent}" (`local.AgentId`))))
  (return (+ (`LearningAgentsRewards.MakeReward` (`self.ePowerReward` (`local.distanceToBallR`) 1000.0 -2.0 5.0) 1.0 "Reward" false null) 0.0 0.0 (`LearningAgentsRewards.MakeRewardOnCondition` _returnvalue 2000.0 "ConditionReward" false null) 0.0 (`LearningAgentsRewards.MakeReward` (`self.ePowerReward` (`/Game/SimBlank/Blueprints/OmniRobot.time` _rewardactor_2) (`/Game/SimBlank/Blueprints/OmniRobot.ballDistanceStart` _rewardactor_2) 75.0 0.24 true) 1.0 "Reward" false null))))

(fn `ResetAgentEpisode`
  (params (AgentId :type Integer))
  (bind _returnvalue (`self.GetAgent` AgentId "/Game/SimBlank/Blueprints/OmniRobot.OmniRobot_C"))
  (`/Engine/EditorBlueprintResources/StandardMacros.IncrementInt` (`/Game/SimBlank/Blueprints/OmniRobot.trainingIteration` _returnvalue)
    (:`  `
      (set `/Game/SimBlank/Blueprints/OmniRobot.time` 0.0 _returnvalue)
      (`/Game/SimBlank/Blueprints/OmniRobot.Event Reset Training` _returnvalue))))