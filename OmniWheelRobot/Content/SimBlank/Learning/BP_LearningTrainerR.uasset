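; Learning Agents trainer that teaches OmniRobot agents to reach a ball and slow down on arrival.
; Reward combines exponential closeness, a penalty for negative speed towards the ball that grows with the robot's iteration count, and a squared-speed penalty near it.
; Episodes end on a short timeout or straying too far; reset relocates the robot and increments that count.
; An iteration-based reward scaling helper exists but the reward graph never calls it.
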(fn `GatherAgentCompletion`
  (params (AgentId :type Integer))
  (returns (OutCompletion :type "ELearningAgentsCompletion Enum"))
  (bind _returnvalue (`self.GetAgent` AgentId "/Game/SimBlank/Blueprints/OmniRobot.OmniRobot_C"))
  (return (`LearningAgentsCompletions.CompletionOr` (`LearningAgentsCompletions.MakeCompletionOnTimeElapsed` (`self.GetEpisodeTime` AgentId) 5.0 "Truncation" "TimeElapsedCompletion" false null) (`LearningAgentsCompletions.MakeCompletionOnLocationDifferenceAboveThreshold` (`SceneComponent.K2_GetComponentLocation` (`/Game/SimBlank/Blueprints/OmniRobot.accurate-body` _returnvalue)) (`/Game/SimBlank/Blueprints/OmniRobot.ballLocation` _returnvalue) 1010.0 "Termination" "LocationDifferenceAboveThresholdCompletion" false null))))

(fn `GatherAgentReward`
  (params (AgentId :type Integer))
  (returns (OutReward :type "Float (single-precision)"))
  (locals (distanceToBall :type "Float (double-precision)" :default 0.0))
  (bind _rewardactor (`self.rewardActor`))
  (bind _speed_towards_ball (`self.Speed Towards Ball`))
  (bind _distancetoball (`local.distanceToBall`))
  (bind _output_get (set `self.rewardActor` (`self.GetAgent` AgentId "/Game/SimBlank/Blueprints/OmniRobot.OmniRobot_C")))
  (bind _speedtowardsball (`/Game/SimBlank/Blueprints/OmniRobot.getSpeedTowardsBall` _output_get))
  (set `self.Speed Towards Ball` _speedtowardsball)
  (set `local.distanceToBall` (`KismetMathLibrary.VSize` (- (`SceneComponent.K2_GetComponentLocation` (`/Game/SimBlank/Blueprints/OmniRobot.accurate-body` _rewardactor)) (`/Game/SimBlank/Blueprints/OmniRobot.ballLocation` _rewardactor))))
  (return (+ (`LearningAgentsRewards.MakeReward` (`KismetMathLibrary.MultiplyMultiply_FloatFloat` 2.718282 (* (/ (`local.distanceToBall`) 1000.0) -2.0)) 10.0 "Reward" false null) (`LearningAgentsRewards.MakeReward` (`KismetMathLibrary.SelectFloat` (* (/ (`/Game/SimBlank/Blueprints/OmniRobot.trainingIteration` (`self.rewardActor`)) 100) _speed_towards_ball) 0.0 (< _speed_towards_ball 0.0)) 1.0 "Reward" false null) (`LearningAgentsRewards.MakeReward` -10.0 (`KismetMathLibrary.SelectFloat` (/ (`KismetMathLibrary.Square` (`self.Speed Towards Ball`)) _distancetoball) 0.0 (< (+ _distancetoball 1e-06) 100.0)) "Reward" false null) 0.0)))

(fn `ResetAgentEpisode`
  (params (AgentId :type Integer))
  (bind _returnvalue (`self.GetAgent` AgentId "/Game/SimBlank/Blueprints/OmniRobot.OmniRobot_C"))
  (`/Game/SimBlank/Blueprints/OmniRobot.Event Reset Location` _returnvalue)
  (`/Engine/EditorBlueprintResources/StandardMacros.IncrementInt` (`/Game/SimBlank/Blueprints/OmniRobot.trainingIteration` _returnvalue)))

(fn `variableReward`
  (params (inputReward :type "Float (double-precision)") (increasing :type Boolean) (halfTime :type Integer))
  (returns (outputReward :type "Float (double-precision)"))
  (bind _returnvalue (/ (* (`/Game/SimBlank/Blueprints/OmniRobot.trainingIteration` (`self.rewardActor`)) 0.62) (`local.halfTime`)))
  (bind _returnvalue_2 (/ (`KismetMathLibrary.Log` (+ _returnvalue 1.0) 10.0) (`KismetMathLibrary.Log` (+ _returnvalue 2.0) 10.0)))
  (return (* (`KismetMathLibrary.SelectFloat` (+ 0.5 _returnvalue_2) (- 1.5 _returnvalue_2) (`local.increasing`)) (`local.inputReward`))))