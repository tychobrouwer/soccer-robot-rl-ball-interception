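; Learning Agents training environment that teaches an OmniRobot to drive to a ball and slow down on arrival.
; Reward combines exponential distance falloff, a penalty for moving away and a large arrival bonus, also logged to the robot's Rewards array.
; Episodes truncate on timeout and terminate when the robot strays too far or arrives slowly.
; Reset triggers the robot's location reset and increments its training iteration.
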(fn `GatherAgentCompletion`
  (params (AgentId :type Integer))
  (returns (OutCompletion :type "ELearningAgentsCompletion Enum"))
  (locals (speedTowardsBallC :type "Float (double-precision)" :default 0.0) (distanceToBallC :type "Float (double-precision)" :default 0.0))
  (bind _returnvalue (`self.GetAgent` AgentId "/Game/SimBlank/Blueprints/OmniRobot.OmniRobot_C"))
  (bind _speedtowardsball (`/Game/SimBlank/Blueprints/OmniRobot.getSpeedTowardsBall` _returnvalue))
  (set `local.speedTowardsBallC` _speedtowardsball)
  (set `local.distanceToBallC` (`KismetMathLibrary.VSize` (- (`SceneComponent.K2_GetComponentLocation` (`/Game/SimBlank/Blueprints/OmniRobot.accurate-body` _returnvalue)) (`/Game/SimBlank/Blueprints/OmniRobot.ballLocation` _returnvalue))))
  (return (`LearningAgentsCompletions.CompletionOr` (`LearningAgentsCompletions.MakeCompletionOnTimeElapsed` (`self.GetEpisodeTime` AgentId) 20.0 "Truncation" "TimeElapsedCompletion" false null) (`LearningAgentsCompletions.MakeCompletionOnCondition` (> (`local.distanceToBallC`) 1000.0) "Termination" "ConditionCompletion" false null) (`LearningAgentsCompletions.MakeCompletionOnCondition` (and (< (`local.distanceToBallC`) 15.0) (< (`local.speedTowardsBallC`) 0.15)) "Termination" "ConditionCompletion" false null) "Running")))

(fn `GatherAgentReward`
  (params (AgentId :type Integer))
  (returns (OutReward :type "Float (single-precision)"))
  (locals (rewardActor :type "/Game/SimBlank/Blueprints/OmniRobot Object Reference") (speedTowardsBallR :type "Float (double-precision)" :default 0.0) (distanceToBallR :type "Float (double-precision)" :default 0.0))
  (bind _rewardactor (`local.rewardActor`))
  (bind _speedtowardsballr (`local.speedTowardsBallR`))
  (bind _returnvalue (+ (`LearningAgentsRewards.MakeReward` (`KismetMathLibrary.MultiplyMultiply_FloatFloat` 2.718282 (* (/ (`local.distanceToBallR`) 1000.0) -2.0)) 10.0 "Reward" false null) (`LearningAgentsRewards.MakeReward` (`KismetMathLibrary.SelectFloat` _speedtowardsballr 0.0 (< _speedtowardsballr 0.0)) 2.0 "Reward" false null) 0.0 (`LearningAgentsRewards.MakeRewardOnCondition` (and (< (`local.distanceToBallR`) 15.0) (< (`local.speedTowardsBallR`) 0.15)) 400.0 "ConditionReward" false null) 0.0))
  (bind _output_get (set `local.rewardActor` (`self.GetAgent` AgentId "/Game/SimBlank/Blueprints/OmniRobot.OmniRobot_C")))
  (bind _speedtowardsball (`/Game/SimBlank/Blueprints/OmniRobot.getSpeedTowardsBall` _output_get))
  (set `local.speedTowardsBallR` _speedtowardsball)
  (set `local.distanceToBallR` (`KismetMathLibrary.VSize` (- (`SceneComponent.K2_GetComponentLocation` (`/Game/SimBlank/Blueprints/OmniRobot.accurate-body` _rewardactor)) (`/Game/SimBlank/Blueprints/OmniRobot.ballLocation` _rewardactor))))
  (`KismetArrayLibrary.Array_Add` (`/Game/SimBlank/Blueprints/OmniRobot.rewards` (`local.rewardActor`)) _returnvalue)
  (return _returnvalue))

(fn `ResetAgentEpisode`
  (params (AgentId :type Integer))
  (bind _returnvalue (`self.GetAgent` AgentId "/Game/SimBlank/Blueprints/OmniRobot.OmniRobot_C"))
  (`/Game/SimBlank/Blueprints/OmniRobot.Event Reset Location` _returnvalue)
  (`/Engine/EditorBlueprintResources/StandardMacros.IncrementInt` (`/Game/SimBlank/Blueprints/OmniRobot.trainingIteration` _returnvalue)))